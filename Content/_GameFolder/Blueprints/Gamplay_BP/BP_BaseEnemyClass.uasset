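; Base enemy Blueprint that shows a health bar widget turned toward the player.
; Every Tick, it casts the Widget component's user widget to AIHealthBar and feeds GetHealth into its progress bar.
; It then yaws the widget along the direction from the enemy to player pawn 0, keeping pitch and roll at zero.
; The rotation is skipped if the cast fails.
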(event `self.ReceiveTick`
  (params (DeltaSeconds :type "Float (single-precision)"))
  ;[1 1 1] Connecting widget and health
  (bind _asaihealth_bar (cast `/Game/_GameFolder/Blueprints/HUD_BP/AIHealthBar` (`WidgetComponent.GetUserWidgetObject` (`self.Widget`))))
  (bind _returnvalue (`self.GetHealth`))
  (`ProgressBar.SetPercent` (`/Game/_GameFolder/Blueprints/HUD_BP/AIHealthBar.ProgressBar_145` _asaihealth_bar) _returnvalue)
  ;[1 1 1] Rotate the Health Bar to Player always
  (`SceneComponent.K2_SetWorldRotation` (`self.Widget`) (`KismetMathLibrary.MakeRotator` 0.0 0.0 (.yaw (`KismetMathLibrary.Conv_VectorToRotator` (- (`self.K2_GetActorLocation` (`GameplayStatics.GetPlayerPawn` 0)) (`self.K2_GetActorLocation`))))) false false))

(fn `UserConstructionScript`)