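; BP_TurretLevel1 is a level 1 turret Blueprint that supplies the aiming behavior toward a target enemy.
; Its LookAtTargetEnemy event points the Turret component's Z axis at a spot a fixed distance along the enemy's forward vector, leading the shot.
; Each call blends from the current world rotation toward that aim by a fixed lerp alpha, easing the turn without using delta time.
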(event `self.ReceiveLookAtTargetEnemy`
  (params (TargetEnemy :type "Actor Object Reference"))
  (bind _turret (`self.Turret`))
  ;[1 1 1] Aim at TargetEnemy
  (bind _output_get (set `self.BP_Turret` (`self.Turret`)))
  (`SceneComponent.K2_SetWorldRotation` _output_get (`KismetMathLibrary.RLerp` (`SceneComponent.K2_GetComponentRotation` _turret) (`KismetMathLibrary.MakeRotFromZ` (`KismetMathLibrary.GetDirectionUnitVector` (`SceneComponent.K2_GetComponentLocation` _turret) (+ (`self.K2_GetActorLocation` TargetEnemy) (* (`self.GetActorForwardVector` TargetEnemy) 100.0)))) 0.33) false false))

(fn `UserConstructionScript`)